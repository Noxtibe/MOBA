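; MOBA player character Blueprint with a "Brise Epouvantail" leap-and-glide ability on the Capacity2 input.
; When grounded and its timer is clear, the input launches the character up and backward from the camera's facing and opens a Gate polled on Tick.
; Once vertical velocity stops rising, low gravity and higher air control create a floaty descent.
; Landing restores both values, resets the timer and closes the Gate.
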(event `self.ReceiveBeginPlay`
  (set `self.Max Walk Speed` (`CharacterMovementComponent.MaxWalkSpeed` (`self.CharacterMovement`))))

(event `self.ReceiveTick`
  (params (DeltaSeconds :type "Float (single-precision)"))
  (`self.eventTickEpouvantail`))

(event `eventTickEpouvantail`
  (bind (_returnvalue_x _returnvalue_y _returnvalue_z) (`KismetMathLibrary.BreakVector` (`self.GetVelocity`)))
  (bind _charactermovement (`self.CharacterMovement`))
  ;[1 0.5224 0 1 42] BRISE EPUVANTAIL
  (`/Engine/EditorBlueprintResources/StandardMacros.Gate` true :!label _label
    (:`Exit`
      (if (<= _returnvalue_z 0.0)
        (set `CharacterMovementComponent.AirControl` 0.5 (`self.CharacterMovement`))
        (set `CharacterMovementComponent.GravityScale` 0.1 _charactermovement)
        (if (`NavMovementComponent.IsMovingOnGround` (`self.CharacterMovement`))
          (set `CharacterMovementComponent.GravityScale` 1.0 _charactermovement)
          (set `CharacterMovementComponent.AirControl` 0.05 _charactermovement)
          (set `self.TImerBriseEpouvantail` 0.0)
          (goto _label :!via `Close`))))))

(event `EnhancedInput|/Game/MOBA_Character/EnhancedInput/Actions/MOBA_Capacity2`
  (params (ActionValue :type Boolean) (ElapsedSeconds :type "Float (double-precision)") (TriggeredSeconds :type "Float (double-precision)") (InputAction :type "InputAction Object Reference" :default "/Game/MOBA_Character/EnhancedInput/Actions/MOBA_Capacity2.MOBA_Capacity2"))
  (bind _charactermovement (`self.CharacterMovement`))
  (bind (_returnvalue_x _returnvalue_y) (`KismetMathLibrary.BreakVector` (`SceneComponent.GetForwardVector` (`self.FirstPersonCameraComponent`))))
  ;[1 0.5224 0 1 42] BRISE EPUVANTAIL
  (:`Triggered`
    (if (<= (`self.TImerBriseEpouvantail`) 0.0)
      (if (`NavMovementComponent.IsMovingOnGround` _charactermovement)
        (`CharacterMovementComponent.AddImpulse` _charactermovement (`KismetMathLibrary.MakeVector` (* _returnvalue_x -1000.0) (* _returnvalue_y -1000.0) 1500.0) true)
        (goto _label :!via `Open`)))))

(fn `UserConstructionScript`)